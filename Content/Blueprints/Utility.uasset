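; Utility functions that serialize a Graph to a JSON string and rebuild a Graph from one.
; GraphToJSON writes the name, each vertex's name and coordinates, and edges as index pairs into the vertex array, found by matching vertex names.
; JSONToGraph decodes through VaRest, recreates the nodes in array order, then links edges by those indices; it does not read back the graph name.
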(fn GraphtoJSON
  (params (Graph :type Graph%20Object%20Reference) (Name :type String))
  (bind _returnvalue (Class|Graph|GetVertexSet Graph))
  (bind _result (Utilities|Set|ToArray _returnvalue))
  (for _array_element _result
    (Utilities|Array|Add (LocalVariables|GetVertices_JSON) (|MakeJson (Class|GraphNode|GetName _array_element) (.x (Class|GraphNode|GetCoordinates _array_element)) (.y (Class|GraphNode|GetCoordinates _array_element)))))
  (bind _returnvalue_2 (Class|Graph|GetEdgeSet Graph))
  (bind _result_2 (Utilities|Set|ToArray _returnvalue_2))
  (for _array_element_2 _result_2
    (bind (_a _b) (CallFunction|FindVerticesforEdgeinJsonArray (LocalVariables|GetVertices_JSON) _array_element_2))
    (Utilities|Array|Add (LocalVariables|GetEdges_JSON) (|MakeJson (Math|Conversions|ToFloat(Integer) _a) (Math|Conversions|ToFloat(Integer) _b))))
  (return (Class|VaRestJsonObject|EncodeJson (|MakeJson (LocalVariables|GetVertices_JSON) (LocalVariables|GetEdges_JSON) Name))))

(fn FindVerticesforEdgeinJsonArray
  (params (Vertices :type Array%20of%20Va%20Rest%20Json%20Object%20Object%20References) (Edge :type Graph%20Edge%20Object%20Reference))
  (for (_array_element _array_index) Vertices
    (if (Utilities|Enum|Equal(Enum) (Class|VaRestJsonObject|GetStringField _array_element "Name") (Class|GraphNode|GetName (Class|GraphEdge|GetStart Edge)))
      (LocalVariables|SetTempA _array_index)
      (elif (Utilities|Enum|Equal(Enum) (Class|VaRestJsonObject|GetStringField _array_element "Name") (Class|GraphNode|GetName (Class|GraphEdge|GetEnd Edge)))
        (LocalVariables|SetTempB _array_index))))
  (return (LocalVariables|GetTempA) (LocalVariables|GetTempB)))

(fn JSONtoGraph
  (params (JSON_String :type String))
  (bind _vertices (LocalVariables|GetVertices))
  (bind _returnvalue (Class|VaRestSubsystem|DecodeJsonObject (|VaRestSubsystem) JSON_String))
  (LocalVariables|SetGraph_JSON _returnvalue)
  (LocalVariables|SetVertices_JSON (Class|VaRestJsonObject|GetObjectArrayField (LocalVariables|GetGraph_JSON) "Vertices"))
  (LocalVariables|SetEdges_JSON (Class|VaRestJsonObject|GetObjectArrayField (LocalVariables|GetGraph_JSON) "Edges"))
  (bind _returnvalue_2 (Class|Graph|CreateGraph))
  (LocalVariables|SetGraph _returnvalue_2)
  (for _array_element (LocalVariables|GetVertices_JSON)
    (bind _returnvalue_3 (Class|Graph|CreateNewNode (LocalVariables|GetGraph) (Class|VaRestJsonObject|GetStringField _array_element "Name") (Math|Vector2D|MakeVector2D (Class|VaRestJsonObject|GetNumberField _array_element "X") (Class|VaRestJsonObject|GetNumberField _array_element "Y"))))
    (Utilities|Array|Add (LocalVariables|GetVertices) _returnvalue_3))
  (for _array_element_2 (LocalVariables|GetEdges_JSON)
    (Class|Graph|CreateNewEdge (LocalVariables|GetGraph) (Utilities|Array|Get(acopy) _vertices (Math|Float|Round (Class|VaRestJsonObject|GetNumberField _array_element_2 "A"))) (Utilities|Array|Get(acopy) _vertices (Math|Float|Round (Class|VaRestJsonObject|GetNumberField _array_element_2 "B")))))
  (return (LocalVariables|GetGraph)))