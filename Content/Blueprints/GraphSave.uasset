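; GraphSave stores named graphs as an array of JSON strings, apparently as save data.
; AddGraph decodes the incoming JSON with VaRest and replaces the stored entry with the same "Name" field, or appends it if none matches.
; GetGraphs decodes each stored string and returns the list of graph names, not the graph contents.
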(fn AddGraph
  (params (GraphAsJSON :type String))
  (bind _returnvalue (Class|VaRestSubsystem|DecodeJsonObject (|VaRestSubsystem) GraphAsJSON))
  (LocalVariables|SetName (Class|VaRestJsonObject|GetStringField _returnvalue "Name"))
  (for (_array_element _array_index) (Variables|Default|GetGraphJSON)
    (bind _returnvalue_2 (Class|VaRestSubsystem|DecodeJsonObject (|VaRestSubsystem) _array_element))
    (if (Utilities|Enum|Equal(Enum) (LocalVariables|GetName) (Class|VaRestJsonObject|GetStringField _returnvalue_2 "Name"))
      (Utilities|Array|SetArrayElem (Variables|Default|GetGraphJSON) _array_index GraphAsJSON true)
      (return)))
  (Utilities|Array|Add (Variables|Default|GetGraphJSON) GraphAsJSON))

(fn GetGraphs
  (for _array_element (Variables|Default|GetGraphJSON)
    (bind _returnvalue (Class|VaRestSubsystem|DecodeJsonObject (|VaRestSubsystem) _array_element))
    (Utilities|Array|Add (LocalVariables|GetAllGraphs) (Class|VaRestJsonObject|GetStringField _returnvalue "Name")))
  (return (LocalVariables|GetAllGraphs)))